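; BP_Foam is a short-lived fire extinguisher foam burst for a 2D side-scroller that damages monsters.
; On spawn it drains the player's FoamTank, plays a sound and destroys itself after a brief delay.
; Every tick it snaps to the player's GunOut transform and spawns a new Foam particle system there.
; Box overlaps call per-type events that cast to Monster_A_2 or Monster_B and subtract Health directly.
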(event OnComponentBeginOverlap(Box)
  (params (OverlappedComponent :type Primitive%20Component%20Object%20Reference) (OtherActor :type Actor%20Object%20Reference) (OtherComp :type Primitive%20Component%20Object%20Reference) (OtherBodyIndex :type Integer) (bFromSweep :type Boolean) (SweepResult :type Hit%20Result%20Structure%20%28by%20ref%29))
  (Utilities|IsValid OtherActor
    (:Is%20Valid
      (CallFunction|DMonA OtherActor)
      (CallFunction|DMonB OtherActor))))

(event Custom|D_MonA
  (params (object :type Actor%20Object%20Reference) (Target :type Monster%20A%20Object%20Reference))
  (bind _asmonster_a_2 (Utilities|Casting|CastToMonster_A_2 object))
  (Variables|/Game/Character/Monster_Characters/Class_A_2/Monster_A_2.Monster_A_2_C|SetHealth _asmonster_a_2 (- (Variables|/Game/Character/Monster_Characters/Class_A_2/Monster_A_2.Monster_A_2_C|GetHealth _asmonster_a_2) 10)))

(event Custom|D_MonB
  (params (Object :type Actor%20Object%20Reference))
  (bind _asmonster_b (Utilities|Casting|CastToMonster_B Object))
  (Variables|/Game/Character/Monster_Characters/Class_B/Monster_B.Monster_B_C|SetHealth _asmonster_b (- (Variables|/Game/Character/Monster_Characters/Class_B/Monster_B.Monster_B_C|GetHealth _asmonster_b) 10)))

(event EventTick
  (params (DeltaSeconds :type Float%20%28single-precision%29))
  (bind _as2dside_scroller_character (Utilities|Casting|CastTo2DSideScrollerCharacter (Game|GetPlayerCharacter 0)))
  (Transformation|SetActorLocationAndRotation (.location (Transformation|GetWorldTransform (Variables|/Game/Character/MainCharacter/2DSideScrollerCharacter.2DSideScrollerCharacter_C|Getgun_out _as2dside_scroller_character))) (.rotation (Transformation|GetWorldTransform (Variables|/Game/Character/MainCharacter/2DSideScrollerCharacter.2DSideScrollerCharacter_C|Getgun_out _as2dside_scroller_character))))
  (Niagara|SpawnSystematLocation "/Game/Extinguisher/Foam.Foam" (Transformation|GetActorLocation) (Transformation|GetActorRotation)))

(event EventBeginPlay
  (bind _as2dside_scroller_character (Utilities|Casting|CastTo2DSideScrollerCharacter (Game|GetPlayerCharacter 0)))
  (Variables|/Game/Character/MainCharacter/2DSideScrollerCharacter.2DSideScrollerCharacter_C|SetFoamTank _as2dside_scroller_character (- (Variables|/Game/Character/MainCharacter/2DSideScrollerCharacter.2DSideScrollerCharacter_C|GetFoamTank _as2dside_scroller_character) 2.0))
  (Audio|PlaySound2D "/Game/Sound/Extin2.Extin2" 1.0 1.0 0.0 0 0)
  (Utilities|FlowControl|Delay 0.6)
  (Actor|DestroyActor))

(fn ConstructionScript)