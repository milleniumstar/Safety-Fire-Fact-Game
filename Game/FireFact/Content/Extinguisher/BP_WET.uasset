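; BP_WET is a short-lived wet extinguisher spray that costs the side-scroller character WetTank charge on spawn and removes itself shortly after.
; Each tick it snaps to the character's GunOut transform and spawns the WET effect system there.
; Box overlaps damage Monster_K actors, then call Death, which plays the fire death sound on every hit and stops the monster's movement once health is depleted.
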(event OnComponentBeginOverlap(Box)
  (params (OverlappedComponent :type Primitive%20Component%20Object%20Reference) (OtherActor :type Actor%20Object%20Reference) (OtherComp :type Primitive%20Component%20Object%20Reference) (OtherBodyIndex :type Integer) (bFromSweep :type Boolean) (SweepResult :type Hit%20Result%20Structure%20%28by%20ref%29))
  (Utilities|IsValid OtherActor
    (:Is%20Valid
      (CallFunction|DMonK OtherActor))))

(event Custom|Death
  (params (Health :type Integer) (Object :type Character%20Object%20Reference))
  (Audio|PlaySound2D "/Game/SoundFX/fire_die_se.fire_die_se" 1.0 1.0 0.0 0 0)
  (if (<= Health 0)
    (Variables|/Script/Engine.CharacterMovementComponent|SetMaxWalkSpeed (Variables|/Script/Engine.Character|GetCharacterMovement Object) 0.0)))

(event Custom|D_MonK
  (params (object :type Actor%20Object%20Reference) (Target :type Monster%20A%20Object%20Reference))
  (bind _asmonster_k (Utilities|Casting|CastToMonster_K object))
  (bind _output_get (Variables|/Game/Character/Monster_Characters/Class_K/Monster_K.Monster_K_C|SetHealth _asmonster_k (- (Variables|/Game/Character/Monster_Characters/Class_K/Monster_K.Monster_K_C|GetHealth _asmonster_k) 10)))
  (CallFunction|Death _output_get _asmonster_k))

(event EventTick
  (params (DeltaSeconds :type Float%20%28single-precision%29))
  (bind _as2dside_scroller_character (Utilities|Casting|CastTo2DSideScrollerCharacter (Game|GetPlayerCharacter 0)))
  (Transformation|SetActorLocationAndRotation (.location (Transformation|GetWorldTransform (Variables|/Game/Character/MainCharacter/2DSideScrollerCharacter.2DSideScrollerCharacter_C|Getgun_out _as2dside_scroller_character))) (.rotation (Transformation|GetWorldTransform (Variables|/Game/Character/MainCharacter/2DSideScrollerCharacter.2DSideScrollerCharacter_C|Getgun_out _as2dside_scroller_character))))
  (Niagara|SpawnSystematLocation "/Game/Extinguisher/WET.WET" (Transformation|GetActorLocation) (Transformation|GetActorRotation)))

(event EventBeginPlay
  (bind _as2dside_scroller_character (Utilities|Casting|CastTo2DSideScrollerCharacter (Game|GetPlayerCharacter 0)))
  (Variables|/Game/Character/MainCharacter/2DSideScrollerCharacter.2DSideScrollerCharacter_C|SetWetTank _as2dside_scroller_character (- (Variables|/Game/Character/MainCharacter/2DSideScrollerCharacter.2DSideScrollerCharacter_C|GetWetTank _as2dside_scroller_character) 2.0))
  (Audio|PlaySound2D "/Game/Sound/Extin2.Extin2" 1.0 1.0 0.0 0 0)
  (Utilities|FlowControl|Delay 0.6)
  (Actor|DestroyActor))

(fn ConstructionScript)