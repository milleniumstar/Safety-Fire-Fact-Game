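; BP_Water is a short-lived water spray actor, apparently from the extinguisher, that plays a sound and destroys itself after a brief delay.
; Every tick it spawns a Water particle system at its own transform.
; Box overlaps run cast-filtered checks: Monster_A_2 loses health, while hitting Monster_C instead stuns and damages the player's side-scroller character.
; An older inline stun, which briefly zeroes walk speed, is left disconnected.
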(event OnComponentBeginOverlap(Box)
  (params (OverlappedComponent :type Primitive%20Component%20Object%20Reference) (OtherActor :type Actor%20Object%20Reference) (OtherComp :type Primitive%20Component%20Object%20Reference) (OtherBodyIndex :type Integer) (bFromSweep :type Boolean) (SweepResult :type Hit%20Result%20Structure%20%28by%20ref%29))
  (Utilities|IsValid OtherActor
    (:Is%20Valid
      (CallFunction|DMonA OtherActor)
      (CallFunction|DMonC OtherActor))))

(event Custom|D_MonC
  (params (object :type Actor%20Object%20Reference) (Target :type Monster%20C%20Object%20Reference))
  (Utilities|Casting|CastToMonster_C object)
  (bind _as2dside_scroller_character (Utilities|Casting|CastTo2DSideScrollerCharacter (Game|GetPlayerCharacter 0)))
  (Default|Stun _as2dside_scroller_character)
  (Variables|/Game/Character/MainCharacter/2DSideScrollerCharacter.2DSideScrollerCharacter_C|SetHealth _as2dside_scroller_character (- (Variables|/Game/Character/MainCharacter/2DSideScrollerCharacter.2DSideScrollerCharacter_C|GetHealth _as2dside_scroller_character) 5.0)))

(event Custom|D_MonA
  (params (object :type Actor%20Object%20Reference) (Target :type Monster%20A%20Object%20Reference))
  (bind _asmonster_a_2 (Utilities|Casting|CastToMonster_A_2 object))
  (Variables|/Game/Character/Monster_Characters/Class_A_2/Monster_A_2.Monster_A_2_C|SetHealth _asmonster_a_2 (- (Variables|/Game/Character/Monster_Characters/Class_A_2/Monster_A_2.Monster_A_2_C|GetHealth _asmonster_a_2) 10)))

(event EventTick
  (params (DeltaSeconds :type Float%20%28single-precision%29))
  (Niagara|SpawnSystematLocation "/Game/Extinguisher/Water.Water" (Transformation|GetActorLocation) (Transformation|GetActorRotation)))

(event EventBeginPlay
  (bind _returnvalue (Audio|SpawnSound2D "/Game/Sound/Water2.Water2" 1.0 1.0 0.0 0))
  (Audio|Components|Audio|Play _returnvalue 0.0)
  (Utilities|FlowControl|Delay 0.6)
  (if (Audio|Components|Audio|IsPlaying _returnvalue)
    (Audio|Components|Audio|Stop _returnvalue))
  (Actor|DestroyActor))

(fn ConstructionScript)