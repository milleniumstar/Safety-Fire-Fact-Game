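; Interactable water present-box actor that opens an info screen for the player in the side-scroller.
; A box trigger shows its Widget component while the 2DSideScrollerCharacter overlaps it and hides it on exit.
; Interacting toggles a lazily created, cached PresentBOX_Water_Widget_BP: opening pauses the game and shows the cursor with game-and-UI input, while closing unpauses and restores game-only input.
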(event OnComponentBeginOverlap(Box)
  (params (OverlappedComponent :type Primitive%20Component%20Object%20Reference) (OtherActor :type Actor%20Object%20Reference) (OtherComp :type Primitive%20Component%20Object%20Reference) (OtherBodyIndex :type Integer) (bFromSweep :type Boolean) (SweepResult :type Hit%20Result%20Structure%20%28by%20ref%29))
  (Utilities|Casting|CastTo2DSideScrollerCharacter OtherActor)
  (Rendering|SetVisibility (Variables|Default|GetWidget) true false))

(event OnComponentEndOverlap(Box)
  (params (OverlappedComponent :type Primitive%20Component%20Object%20Reference) (OtherActor :type Actor%20Object%20Reference) (OtherComp :type Primitive%20Component%20Object%20Reference) (OtherBodyIndex :type Integer))
  (Utilities|Casting|CastTo2DSideScrollerCharacter OtherActor)
  (Rendering|SetVisibility (Variables|Default|GetWidget) false false))

(event Custom|Open_PresentBOX_WaterInfo_Text
  (bind _returnvalue (Game|GetPlayerController 0))
  ;[1 1 1] To_OP_Widgets
  (Utilities|IsValid (Variables|Default|GetWater_Info_REF)
    (:Is%20Valid
      _)
    (:Is%20Not%20Valid
      (bind _returnvalue_2 (UserInterface|CreateWidget "/Game/Extinguisher/Present_BOX/Water/PresentBOX_Water_Widget_BP.PresentBOX_Water_Widget_BP_C"))
      (Variables|Default|SetWater_Info_REF _returnvalue_2)))
  (if (Game|IsGamePaused)
    (Widget|RemovefromParent (Variables|Default|GetWater_Info_REF))
    (Game|SetGamePaused false)
    (Variables|/Script/Engine.PlayerController|SetbShowMouseCursor _returnvalue false)
    (Input|SetInputModeGameOnly _returnvalue)
    (else
      (UserInterface|Viewport|AddtoViewport (Variables|Default|GetWater_Info_REF) 0)
      (Game|SetGamePaused true)
      (Variables|/Script/Engine.PlayerController|SetbShowMouseCursor _returnvalue true)
      (Input|SetInputModeGameandUI _returnvalue 0 "LockInFullscreen" false))))

(event EventBeginPlay)

(event Collision|EventActorBeginOverlap
  (params (OtherActor :type Actor%20Object%20Reference)))

(event EventTick
  (params (DeltaSeconds :type Float%20%28single-precision%29)))

(fn ConstructionScript)

(fn InteractBP
  (params (Interactor :type Character%20Object%20Reference))
  (CallFunction|OpenPresentBOXWaterInfoText)
  (return false))