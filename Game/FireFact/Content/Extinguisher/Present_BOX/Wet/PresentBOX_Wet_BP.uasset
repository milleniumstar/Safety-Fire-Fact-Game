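; PresentBOX_Wet_BP is an interactable wet-type present box in the extinguisher content that toggles an info widget when interacted with.
; Its InteractBP implementation calls a custom event, which lazily creates and caches PresentBOX_DryWet_Widget_BP.
; The game's pause state drives the toggle: unpaused, it shows the widget, pauses and enables the cursor with Game-and-UI input; paused, it reverses all of that.
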(event Custom|Open_PresentBOX_WetInfo_Text
  (bind _returnvalue (Game|GetPlayerController 0))
  ;[1 1 1] To_OP_Widgets
  (Utilities|IsValid (Variables|Default|GetWet_REF)
    (:Is%20Valid
      _)
    (:Is%20Not%20Valid
      (bind _returnvalue_2 (UserInterface|CreateWidget "/Game/Extinguisher/Present_BOX/Wet/PresentBOX_DryWet_Widget_BP.PresentBOX_DryWet_Widget_BP_C"))
      (Variables|Default|SetWet_REF _returnvalue_2)))
  (if (Game|IsGamePaused)
    (Widget|RemovefromParent (Variables|Default|GetWet_REF))
    (Game|SetGamePaused false)
    (Variables|/Script/Engine.PlayerController|SetbShowMouseCursor _returnvalue false)
    (Input|SetInputModeGameOnly _returnvalue)
    (else
      (UserInterface|Viewport|AddtoViewport (Variables|Default|GetWet_REF) 0)
      (Game|SetGamePaused true)
      (Variables|/Script/Engine.PlayerController|SetbShowMouseCursor _returnvalue true)
      (Input|SetInputModeGameandUI _returnvalue 0 "LockInFullscreen" false))))

(event EventBeginPlay)

(event Collision|EventActorBeginOverlap
  (params (OtherActor :type Actor%20Object%20Reference)))

(event EventTick
  (params (DeltaSeconds :type Float%20%28single-precision%29)))

(fn ConstructionScript)

(fn InteractBP
  (params (Interactor :type Character%20Object%20Reference))
  (CallFunction|OpenPresentBOXWetInfoText)
  (return false))