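; Fireball projectile actor for a 2D side-scroller that hurts and knocks back characters it touches.
; When its sphere overlaps a 2DSideScrollerCharacter, it plays a hit sound and subtracts a fixed amount from that character's Health.
; It launches the character upward and along X in the fireball's direction of travel, judged by the sign of its velocity, then destroys itself.
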(event OnComponentBeginOverlap(Sphere)
  (params (OverlappedComponent :type Primitive%20Component%20Object%20Reference) (OtherActor :type Actor%20Object%20Reference) (OtherComp :type Primitive%20Component%20Object%20Reference) (OtherBodyIndex :type Integer) (bFromSweep :type Boolean) (SweepResult :type Hit%20Result%20Structure%20%28by%20ref%29))
  (bind _as2dside_scroller_character (Utilities|Casting|CastTo2DSideScrollerCharacter OtherActor))
  (Audio|PlaySound2D "/Game/Sound/Hit.Hit" 1.0 1.0 0.0 0 0)
  (Variables|/Game/Character/MainCharacter/2DSideScrollerCharacter.2DSideScrollerCharacter_C|SetHealth _as2dside_scroller_character (- (Variables|/Game/Character/MainCharacter/2DSideScrollerCharacter.2DSideScrollerCharacter_C|GetHealth _as2dside_scroller_character) 1e+01))
  (if (>= (.x (Transformation|GetVelocity)) 0.0)
    (Character|LaunchCharacter _as2dside_scroller_character "300.000000, 0,200.000000" false true)
    (else
      (Character|LaunchCharacter _as2dside_scroller_character "-300.000000, 0,200.000000" false true)))
  (Actor|DestroyActor))

(fn ConstructionScript)